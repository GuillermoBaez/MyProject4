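; Game mode that tracks a count of boxes, MNBoxes, as they explode.
; On BeginPlay it binds a custom event to the BoxExploswww dispatcher and adds a MyHud widget to the viewport.
; The bound event calls BoxExplosion to decrement the count, which GetBoxes exposes.
; Tick checks whether boxes remain but takes no action.
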(event Custom|CustomEvent_0
  (CallFunction|BoxExplosion))

(event EventBeginPlay
  (EventDispatchers|BindEventtoBoxExploswww (delegate Custom|CustomEvent_0))
  (bind _returnvalue (UserInterface|CreateWidget "/Game/Blueprints/myHud.myHud_C"))
  (UserInterface|Viewport|AddtoViewport _returnvalue 0))

(event EventTick
  (params (DeltaSeconds :type Float%20%28single-precision%29))
  (if (> (Variables|Default|Getm_nBoxes) 0)
    _))

(event Custom|boxExplosion
  (Variables|Default|Setm_nBoxes (- (Variables|Default|Getm_nBoxes) 1)))

(fn ConstructionScript)

(fn GetBoxes
  (return (Variables|Default|Getm_nBoxes)))